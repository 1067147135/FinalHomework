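; NewAIBP is a simple AI character with movement events and a proximity-triggered animation.
; AIFollow moves it toward the player pawn, while AIMove sends it to a random navigable point nearby.
; Overlap of its SphereCollision with MyCharactorBP plays MyMontage, and ending the overlap stops it.
; BeginPlay is empty and the looping AIFollow timer is disconnected, so nothing here triggers either movement event.
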(event OnComponentBeginOverlap(SphereCollision)
  (params (OverlappedComponent :type Primitive%20Component%20Object%20Reference) (OtherActor :type Actor%20Object%20Reference) (OtherComp :type Primitive%20Component%20Object%20Reference) (OtherBodyIndex :type Integer) (bFromSweep :type Boolean) (SweepResult :type Hit%20Result%20Structure%20%28by%20ref%29))
  (Utilities|Casting|CastToMyCharactorBP OtherActor)
  (Animation|PlayAnimMontage "/Game/MyCharactor/MyMontage.MyMontage" 1.0 "Default"))

(event OnComponentEndOverlap(SphereCollision)
  (params (OverlappedComponent :type Primitive%20Component%20Object%20Reference) (OtherActor :type Actor%20Object%20Reference) (OtherComp :type Primitive%20Component%20Object%20Reference) (OtherBodyIndex :type Integer))
  (Utilities|Casting|CastToMyCharactorBP OtherActor)
  (Animation|StopAnimMontage "/Game/MyCharactor/MyMontage.MyMontage"))

(event Custom|AIFollow
  (AI|AIMoveTo self "0, 0, 0" (Game|Player|GetPlayerPawn 0) 5.0 true))

(event Custom|AIMove
  (AI|AIMoveTo self (.RandomLocation (Class|NavigationSystemV1|GetRandomPointinNavigableRadius (Transformation|GetActorLocation) 5e+03 0 0)) 0 5.0 true))

(event EventBeginPlay)

(fn ConstructionScript)